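; Customer spawner that creates customers at a spawn point and manages their queue along a fixed set of spots.
; Tick counts down a randomized delay, then spawns a customer with a random item and display, targeting the next free spot, unless the queue is full.
; DequeueCustomer shifts everyone behind the departing customer forward one spot and removes that customer from the list.
; A delayed LeaveArea call on the first customer is left unconnected.
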(event Custom|DequeueCustomer
  (params (Customer :type BP%20Customer%20Object%20Reference))
  (bind _currentcustomers (Variables|Default|GetCurrentCustomers))
  (for (_array_element _array_index) _currentcustomers
    (if (> _array_index (Utilities|Array|FindItem _currentcustomers Customer))
      (Default|UpdatePosition _array_element (Utilities|Array|Get(acopy) (Variables|Default|GetCustomerSpots) (- _array_index 1)))))
  (Utilities|Array|RemoveItem (Variables|Default|GetCurrentCustomers) Customer))

(event EventTick
  (params (DeltaSeconds :type Float%20%28single-precision%29))
  (bind _allitems (Variables|Default|GetAllItems))
  (bind _returnvalue (Utilities|Array|Length _allitems))
  (bind _returnvalue_2 (Math|Random|RandomInteger _returnvalue))
  (bind _output_get (Variables|Default|SetSpawnDelay (- (Variables|Default|GetSpawnDelay) DeltaSeconds)))
  (if (<= _output_get 0.0)
    (CallFunction|SetSpawnDelay)
    (if (< (Utilities|Array|Length (Variables|Default|GetCurrentCustomers)) (Utilities|Array|Length (Variables|Default|GetCustomerSpots)))
      (bind _returnvalue_3 (Game|SpawnActorfromClass (Variables|Default|GetCustomer) (Transformation|GetWorldTransform (Variables|Default|GetSpawnPoint)) "AdjustIfPossibleButAlwaysSpawn" "MultiplyWithRoot" 0 (Utilities|Array|Get(acopy) (Variables|Default|GetAllItemDisplays) _returnvalue_2) (Utilities|Array|Get(acopy) (Variables|Default|GetAllItems) _returnvalue_2) (Utilities|Array|Get(acopy) (Variables|Default|GetCustomerSpots) (Utilities|Array|Length (Variables|Default|GetCurrentCustomers))) 0))
      (Utilities|Array|Add (Variables|Default|GetCurrentCustomers) _returnvalue_3))))

(event EventBeginPlay
  (CallFunction|SetSpawnDelay))

(fn ConstructionScript)

(fn SetSpawnDelay
  (Variables|Default|SetSpawnDelay (Math|Random|RandomFloatinRange 5.0 1e+01)))