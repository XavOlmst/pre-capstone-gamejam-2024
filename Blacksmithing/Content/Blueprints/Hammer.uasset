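; Hammer actor for a sword-forging timing minigame, started with a Sword reference while hiding the first-person character's tool.
; A looping timeline ping-pongs the hammer along Y between the sword's Top and Bottom components.
; Swing reports the current Y to the sword's CheckHammer, then plays a roll timeline forward and back, ignoring repeat swings until done.
; EndMinigame stops the movement and restores the transform saved by SetOriginalTransform.
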(event Custom|SetOriginalTransform
  (bind _returnvalue (Transformation|GetActorTransform))
  (Variables|Default|SetoriginalPos (.location _returnvalue))
  (Variables|Default|SetoriginalRot (.rotation _returnvalue)))

(event Custom|StartMinigame
  (params (Sword :type Sword%20Object%20Reference))
  (bind _returnvalue (Transformation|GetActorLocation))
  (bind _returnvalue_2 (Transformation|GetActorLocation))
  (bind _output_get (Variables|Default|Setsword Sword))
  (bind _asbp_first_person_character (Utilities|Casting|CastToBP_FirstPersonCharacter (Game|GetPlayerCharacter 0)))
  (Default|TurnToolInvisible _asbp_first_person_character)
  (Variables|Default|SetoriginalY (.y (Transformation|GetActorLocation _output_get)))
  (bind _move (Timeline|MoveBackAndForth PlayFromStart)
    (:Update
      (if (Variables|Default|GetposDirection)
        (Transformation|SetActorLocation (Math|Vector|MakeVector (.x _returnvalue_2) (Math|Float|Lerp (.y (Transformation|GetWorldLocation (Variables|/Game/Blueprints/Sword.Sword_C|GetTop (Variables|Default|Getsword)))) (.y (Transformation|GetWorldLocation (Variables|/Game/Blueprints/Sword.Sword_C|GetBottom (Variables|Default|Getsword)))) _move) (.z _returnvalue_2)) false false)
        (else
          (Transformation|SetActorLocation (Math|Vector|MakeVector (.x _returnvalue) (Math|Float|Lerp (.y (Transformation|GetWorldLocation (Variables|/Game/Blueprints/Sword.Sword_C|GetBottom (Variables|Default|Getsword)))) (.y (Transformation|GetWorldLocation (Variables|/Game/Blueprints/Sword.Sword_C|GetTop (Variables|Default|Getsword)))) _move) (.z _returnvalue)) false false))))
    (:Finished
      (if (Variables|Default|GetposDirection)
        (Variables|Default|SetposDirection false)
        (else
          (Variables|Default|SetposDirection true)))
      (Components|Timeline|PlayfromStart (Variables|Default|GetMoveBackAndForth)))))

(event Custom|EndMinigame
  (Audio|Components|Audio|Stop (Variables|Default|GetMoveBackAndForth))
  (Transformation|SetActorTransform (Math|Transform|MakeTransform (Variables|Default|GetoriginalPos) (Variables|Default|GetoriginalRot) "1.000000,1.000000,1.000000"))
  (Variables|Default|Setswinging false)
  (Variables|Default|SetrotDir false)
  (Variables|Default|SetposDirection false))

(event Custom|Swing
  (bind _returnvalue (Transformation|GetActorRotation))
  (if (not (Variables|Default|Getswinging))
    (Variables|Default|Setswinging true)
    (Default|CheckHammer (Variables|Default|Getsword) (.y (Transformation|GetActorLocation)))
    (Variables|Default|SetogRotX (.roll (Transformation|GetActorRotation)))
    (Variables|Default|SetrotDir true)
    (bind _rotateovertime (Timeline|SwingRotation PlayFromStart)
      (:Update
        (if (Variables|Default|GetrotDir)
          (Transformation|SetActorRotation (Math|Rotator|MakeRotator (Math|Float|Lerp (+ (Variables|Default|GetogRotX) (Variables|Default|GetminRotation)) (+ (Variables|Default|GetogRotX) (Variables|Default|GetmaxRotation)) _rotateovertime) (.pitch _returnvalue) (.yaw _returnvalue)))
          (else
            (Transformation|SetActorRotation (Math|Rotator|MakeRotator (Math|Float|Lerp (+ (Variables|Default|GetogRotX) (Variables|Default|GetmaxRotation)) (+ (Variables|Default|GetogRotX) (Variables|Default|GetminRotation)) _rotateovertime) (.pitch _returnvalue) (.yaw _returnvalue))))))
      (:Finished
        (if (Variables|Default|GetrotDir)
          (Variables|Default|SetrotDir false)
          (Components|Timeline|PlayfromStart (Variables|Default|GetSwingRotation))
          (else
            (Variables|Default|Setswinging false)))))))

(event EventBeginPlay
  (Variables|Default|Setswinging false)
  (Variables|Default|SetrotDir false)
  (Variables|Default|SetposDirection false))

(fn ConstructionScript)