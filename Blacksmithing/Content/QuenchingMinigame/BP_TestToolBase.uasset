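; Test base tool for the quenching minigame, tracking a sword's temperature and repair state.
; HeatTool increments temperature by a frame-scaled rate when within a small margin of ambient, otherwise snaps to ambient, flagging Melted past the melting point.
; CoolTool subtracts temperature with a minimum check, and IsWorkable tests the working-to-melting range.
; Broken, dull and sharpened states are represented by meshes in ToolMeshs, swapped by RepairTool and SharpenTool.
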(event Custom|CoolTool
  (params (TempReduction :type Float%20%28double-precision%29))
  (if (<= (Variables|Default|GetCurrentTemp) (Variables|Default|GetMinTemp))
    (Variables|Default|SetCurrentTemp (Variables|Default|GetMinTemp))
    (else
      (bind _output_get (Variables|Default|SetCurrentTemp (- (Variables|Default|GetCurrentTemp) TempReduction)))
      (Development|PrintString (Utilities|String|ToString(Float) _output_get)))))

(event Custom|RepairTool
  (Components|StaticMesh|SetStaticMesh (Variables|Default|Getsword_broken) (Utilities|Array|Get(acopy) (Variables|Default|GetToolMeshs) 1)))

(event Custom|SharpenTool
  (Components|StaticMesh|SetStaticMesh (Variables|Default|Getsword_broken) (Utilities|Array|Get(acopy) (Variables|Default|GetToolMeshs) 2)))

(event Custom|HeatTool
  (params (AmbientTemp :type Float%20%28double-precision%29))
  (if (< (Math|Float|Absolute(Float) (- AmbientTemp (Variables|Default|GetCurrentTemp))) 5.0)
    (bind _output_get (Variables|Default|SetCurrentTemp (+ (Variables|Default|GetCurrentTemp) (* (Variables|Default|GetHeatingRate) (Utilities|Time|GetWorldDeltaSeconds)))))
    (Development|PrintString (Utilities|String|ToString(Float) _output_get))
    (if (> _output_get (Variables|Default|GetMeltingTemp))
      (Variables|Default|SetMelted true))
    (else
      (Variables|Default|SetCurrentTemp AmbientTemp))))

(fn ConstructionScript)

(fn IsWorkable
  (return (and (< (Variables|Default|GetCurrentTemp) (Variables|Default|GetMeltingTemp)) (> (Variables|Default|GetCurrentTemp) (Variables|Default|GetWorkingTemp)))))

(fn IsBroken
  (return (== (Utilities|Array|Get(acopy) (Variables|Default|GetToolMeshs)) (Variables|/Script/Engine.StaticMeshComponent|GetStaticMesh (Variables|Default|Getsword_broken)))))

(fn IsDull
  (return (== (Utilities|Array|Get(acopy) (Variables|Default|GetToolMeshs) 1) (Variables|/Script/Engine.StaticMeshComponent|GetStaticMesh (Variables|Default|Getsword_broken)))))