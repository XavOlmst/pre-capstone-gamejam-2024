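; BP_QuenchingBarrel is the barrel for the quenching minigame, where the player cools a held tool.
; StartMinigame toggles: it places and orients the tool at a start point and disables player movement, or stops, restores movement and resets the tool.
; While QuenchTool sets cooling, Tick snaps the tool to the end point and cools it over time, otherwise returning it.
; A sphere overlap tracks player proximity and stops the minigame on exit.
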(event OnComponentBeginOverlap(Sphere)
  (params (OverlappedComponent :type Primitive%20Component%20Object%20Reference) (OtherActor :type Actor%20Object%20Reference) (OtherComp :type Primitive%20Component%20Object%20Reference) (OtherBodyIndex :type Integer) (bFromSweep :type Boolean) (SweepResult :type Hit%20Result%20Structure%20%28by%20ref%29))
  ;[1 1 1] Determine players proximity to barrel
  (if (== OtherActor (Variables|Default|GetPlayer))
    (Variables|Default|SetnearQuench true)))

(event OnComponentEndOverlap(Sphere)
  (params (OverlappedComponent :type Primitive%20Component%20Object%20Reference) (OtherActor :type Actor%20Object%20Reference) (OtherComp :type Primitive%20Component%20Object%20Reference) (OtherBodyIndex :type Integer))
  ;[1 1 1] Determine players proximity to barrel
  (if (== OtherActor (Variables|Default|GetPlayer))
    (Variables|Default|SetnearQuench false)
    (CallFunction|StopMinigame)))

(event Custom|StartMinigame
  (params (Tool :type BP%20Test%20Tool%20Base%20Object%20Reference))
  (bind _toolstartpos (Variables|Default|GetToolStartPos))
  (bind _returnvalue (Transformation|GetWorldLocation _toolstartpos))
  (if (Variables|Default|GetinMinigame)
    (CallFunction|StopMinigame)
    (else
      (bind _output_get (Variables|Default|SetCoolingTool Tool))
      (Transformation|SetWorldLocation (Variables|/Game/QuenchingMinigame/BP_TestToolBase.BP_TestToolBase_C|GetDefaultSceneRoot _output_get) (Transformation|GetWorldLocation (Variables|Default|GetToolStartPos)) false false)
      (Transformation|SetWorldRotation (Variables|/Script/Engine.Actor|GetRootComponent (Variables|Default|GetCoolingTool)) (Math|Rotator|FindLookatRotation _returnvalue (+ _returnvalue (Math|Vector|GetForwardVector _toolstartpos))) false false)
      (Variables|Default|SetinMinigame true)
      (Components|Activation|SetActive (Pawn|GetMovementComponent (Variables|Default|Getplayer)) false false))))

(event Custom|QuenchTool
  (Variables|Default|SetIsCooling true))

(event Custom|StopQuench
  (Variables|Default|SetIsCooling false))

(event Custom|StopMinigame
  (Variables|Default|SetCoolingTool 0)
  (Variables|Default|SetinMinigame false)
  (Components|Activation|SetActive (Pawn|GetMovementComponent (Variables|Default|Getplayer)) true false)
  (bind _asbp_first_person_character (Utilities|Casting|CastToBP_FirstPersonCharacter (Game|GetPlayerCharacter 0)))
  (Default|ResetTool _asbp_first_person_character))

(event EventTick
  (params (DeltaSeconds :type Float%20%28single-precision%29))
  (if (Variables|Default|GetinMinigame)
    (if (Variables|Default|GetIsCooling)
      (Default|CoolTool (Variables|Default|GetCoolingTool) (* DeltaSeconds (Variables|Default|GetCoolingRate)))
      (Transformation|SetActorLocation (Variables|Default|GetCoolingTool) (Transformation|GetWorldLocation (Variables|Default|GetToolEndPos)) false false)
      (else
        (Transformation|SetActorLocation (Variables|Default|GetCoolingTool) (Transformation|GetWorldLocation (Variables|Default|GetToolStartPos)) false false)))))

(event EventBeginPlay
  (bind _asbp_first_person_character (Utilities|Casting|CastToBP_FirstPersonCharacter (Game|Player|GetPlayerPawn 0)))
  (Variables|Default|Setplayer _asbp_first_person_character))

(fn ConstructionScript)