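; Anvil actor that hosts a sword-hammering minigame for the first-person player.
; Overlapping its trigger spawns a Hammer attached to the player and leaving destroys it.
; HammerTime toggles via FlipFlop between locking movement with a top-down view, spawning a Sword and starting the Hammer's minigame, and ending it.
; EndMinigame restores the player, destroys the Sword and swaps the current tool's broken-sword mesh to the dull one.
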(event OnComponentBeginOverlap(Trigger)
  (params (OverlappedComponent :type Primitive%20Component%20Object%20Reference) (OtherActor :type Actor%20Object%20Reference) (OtherComp :type Primitive%20Component%20Object%20Reference) (OtherBodyIndex :type Integer) (bFromSweep :type Boolean) (SweepResult :type Hit%20Result%20Structure%20%28by%20ref%29))
  (bind _player (Variables|Default|Getplayer))
  (if (== OtherActor _player)
    (Variables|Default|SetnearAnvil true)
    (bind _returnvalue (Game|SpawnActorfromClass "/Game/Blueprints/Hammer.Hammer_C" (Transformation|GetActorTransform _player) "Undefined" "MultiplyWithRoot" 0 0))
    (bind _output_get (Variables|Default|Sethammer _returnvalue))
    (Transformation|AttachActorToActor _output_get (Variables|Default|Getplayer) "" "SnapToTarget" "SnapToTarget" "SnapToTarget" true)
    (Transformation|SetActorTransform (Variables|Default|Gethammer) (Math|Transform|MakeTransform (+ (.location (Transformation|GetActorTransform (Variables|Default|Gethammer))) "75.000000,75.000000,50.000000") "0.000000,90.000000,-45.000000" (.scale (Transformation|GetActorTransform (Variables|Default|Gethammer)))))
    (Default|SetOriginalTransform (Variables|Default|Gethammer))))

(event OnComponentEndOverlap(Trigger)
  (params (OverlappedComponent :type Primitive%20Component%20Object%20Reference) (OtherActor :type Actor%20Object%20Reference) (OtherComp :type Primitive%20Component%20Object%20Reference) (OtherBodyIndex :type Integer))
  (bind _hammer (Variables|Default|Gethammer))
  (if (== OtherActor (Variables|Default|Getplayer))
    (if (Utilities|IsValid _hammer)
      (Actor|DestroyActor _hammer)
      (Variables|Default|SetnearAnvil false))))

(event Custom|Hammer%20Time
  (params (tool :type BP%20Test%20Tool%20Base%20Object%20Reference))
  (bind _player (Variables|Default|Getplayer))
  (bind _player_2 (Variables|Default|Getplayer))
  (bind _top1 (Variables|Default|GetTop1))
  (bind _hammer (Variables|Default|GetHammer))
  (bind _returnvalue (Transformation|GetWorldLocation _top1))
  (bind _returnvalue_2 (Transformation|GetActorLocation _hammer))
  (bind _firstpersoncameracomponent (Variables|/Script/Blacksmithing.BlacksmithingCharacter|GetFirstPersonCameraComponent _player))
  (bind _returnvalue_3 (+ _returnvalue "-50.000000,0.000000,100.000000"))
  (bind _returnvalue_4 (Math|Rotator|FindLookatRotation _returnvalue_3 _returnvalue))
  (Variables|Default|SetcurrentTool tool)
  (if (Utilities|IsValid (Variables|Default|Gethammer))
    (Utilities|FlowControl|FlipFlop
      (:A
        (Input|SetIgnoreLookInput (Pawn|GetController (Variables|Default|Getplayer)) false)
        (Components|Activation|SetActive (Pawn|GetMovementComponent (Variables|Default|Getplayer)) false false)
        (Variables|Default|SetogPos (Transformation|GetActorLocation _player_2))
        (Variables|Default|SetogRot (Transformation|GetActorRotation _player_2))
        (Variables|/Script/Engine.CameraComponent|SetbUsePawnControlRotation _firstpersoncameracomponent false)
        (Transformation|SetRelativeRotation _firstpersoncameracomponent "0, 0, 0" false false)
        (Transformation|SetActorLocationAndRotation (Variables|Default|Getplayer) _returnvalue_3 _returnvalue_4)
        (Default|RotateControls (Variables|Default|Getcontrols) _returnvalue_4)
        (bind _returnvalue_5 (Game|SpawnActorfromClass "/Game/Blueprints/Sword.Sword_C" (Math|Transform|MakeTransform (Transformation|GetWorldLocation (Variables|Default|GetTop)) "0.000000,0.000000,90.000000" "1.000000,1.000000,1.000000") "Undefined" "MultiplyWithRoot" 0 0))
        (bind _output_get (Variables|Default|Setsword _returnvalue_5))
        (Variables|/Game/Blueprints/Sword.Sword_C|Setanvil _output_get self)
        (Transformation|SetActorTransform (Variables|Default|Gethammer) (Math|Transform|MakeTransform (Math|Vector|MakeVector (+ (.x _returnvalue_2) 25.0) (.y (Transformation|GetWorldLocation (Variables|/Game/Blueprints/Sword.Sword_C|GetBottom _output_get))) (.z _returnvalue_2)) (Transformation|GetActorRotation _hammer) "0.500000,0.500000,0.500000"))
        (Default|StartMinigame (Variables|Default|Gethammer) (Variables|Default|Getsword))
        (Variables|Default|SethammerTime true))
      (:B
        (CallFunction|EndMinigame)))))

(event Custom|SwingHammer
  (Default|Swing (Variables|Default|Gethammer)))

(event Custom|EndMinigame
  (Components|Activation|SetActive (Pawn|GetMovementComponent (Variables|Default|Getplayer)) true false)
  (Transformation|SetActorTransform (Variables|Default|Getplayer) (Math|Transform|MakeTransform (Variables|Default|GetogPos) (Variables|Default|GetogRot) "1.000000,1.000000,1.000000"))
  (Default|RotateControls (Variables|Default|Getcontrols) (Variables|Default|GetogRot))
  (Variables|/Script/Engine.CameraComponent|SetbUsePawnControlRotation (Variables|/Script/Blacksmithing.BlacksmithingCharacter|GetFirstPersonCameraComponent (Variables|Default|Getplayer)) true)
  (Actor|DestroyActor (Variables|Default|Getsword))
  (Default|EndMinigame (Variables|Default|Gethammer))
  (Variables|Default|SethammerTime false)
  (Input|SetIgnoreLookInput (Pawn|GetController (Variables|Default|Getplayer)) false)
  ;[1 1 1] set sword mesh here
  (Components|StaticMesh|SetStaticMesh (Variables|/Game/QuenchingMinigame/BP_TestToolBase.BP_TestToolBase_C|Getsword_broken (Variables|Default|GetcurrentTool)) "/Game/meshes/sword_dull.sword_dull"))

(event EventBeginPlay
  (bind _asbp_first_person_character (Utilities|Casting|CastToBP_FirstPersonCharacter (Game|Player|GetPlayerPawn 0)))
  (Variables|Default|Setplayer _asbp_first_person_character))

(fn ConstructionScript)