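; Customer pawn that walks to a target spot, carries a spawned item and shows a widget of the item it requests.
; BeginPlay attaches the item, sets the widget image and moves via AIMoveTo, revealing the widget on arrival; Tick turns it toward the player.
; UpdatePosition re-targets movement.
; LeaveArea hides the widget, heads to BP_CustomerExit and dequeues from BP_CustomerSpawner as movement starts, destroying itself if the move fails.
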(event Custom|LeaveArea
  (Rendering|SetVisibility (Variables|Default|GetRequestItem) false false)
  (bind _returnvalue (Actor|GetActorOfClass "/Game/CustomerInteractions/BP_CustomerExit.BP_CustomerExit_C"))
  (Utilities|IsValid _returnvalue
    (:Is%20Valid
      (bind _movementresult (AI|AIMoveTo self "0, 0, 0" _returnvalue 5.0 false)
        (:then
          (bind _returnvalue_2 (Actor|GetActorOfClass "/Game/CustomerInteractions/BP_CustomerSpawner.BP_CustomerSpawner_C"))
          (Default|DequeueCustomer _returnvalue_2 self)
          (Development|PrintString "Customer Left"))
        (:OnFail
          ;[1 1 1] Debug Info for when things fail
          (Development|PrintString (Utilities|String|EnumtoString _movementresult))
          (Actor|DestroyActor))))
    (:Is%20Not%20Valid
      (Development|PrintString "Exit not found"))))

(event Custom|UpdatePosition
  (params (Target :type Actor%20Object%20Reference))
  (AI|AIMoveTo self "0, 0, 0" Target 5.0 false
    (:then
      (Rendering|SetVisibility (Variables|Default|GetRequestItem) true false))))

(event EventBeginPlay
  (bind _scene (Variables|Default|GetScene))
  (bind _returnvalue (Game|SpawnActorfromClass (Variables|Default|GetItem) (Transformation|GetWorldTransform _scene) "Undefined" "MultiplyWithRoot" 0 0))
  (bind _output_get (Variables|Default|SetHeldTool _returnvalue))
  (Transformation|AttachComponentToComponent _output_get _scene "None" "SnapToTarget" "SnapToTarget" "SnapToTarget" true)
  (bind _aswb_item_display (Utilities|Casting|CastToWB_ItemDisplay (UserInterface|GetWidget (Variables|Default|GetRequestItem)))
    (:then
      (Variables|/Game/CustomerInteractions/UI/WB_ItemDisplay.WB_ItemDisplay_C|SetImageToDisplay _aswb_item_display (Variables|Default|GetItemDisplay))
      (AI|AIMoveTo self "0, 0, 0" (Variables|Default|GetTargetLocation) 5.0 false
        (:OnSuccess
          (Rendering|SetVisibility (Variables|Default|GetRequestItem) true false))))
    (:CastFailed
      (Development|PrintString "Could not cast to ITEM DISPLAY WIDGET" true true "(R=1.000000,G=0.000000,B=0.042729,A=1.000000)"))))

(event EventTick
  (params (DeltaSeconds :type Float%20%28single-precision%29))
  (bind _returnvalue (Actor|GetActorOfClass "/Game/FirstPerson/Blueprints/BP_FirstPersonCharacter.BP_FirstPersonCharacter_C"))
  (Transformation|SetWorldRotation (Variables|Default|GetRequestItem) (Math|Rotator|FindLookatRotation (Transformation|GetWorldLocation (Variables|Default|GetRequestItem)) (Transformation|GetWorldLocation (Variables|/Script/Engine.Character|GetCapsuleComponent _returnvalue))) false false))

(fn ConstructionScript)