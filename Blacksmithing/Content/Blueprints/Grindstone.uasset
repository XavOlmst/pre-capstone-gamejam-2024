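; Grindstone station that runs a timing minigame on the tool passed to it and tracks whether the player is near.
; Tick bounces a progress value across a WB_GrindstoneUI bar until accumulated grind time reaches the limit.
; StartGrinding adds time regardless of accuracy, moves the tool to the Top1 point and tints the bar green or red by the click-area angle range.
; StopGrinding returns the tool to Top and resets the tint.
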(event OnComponentEndOverlap(Trigger)
  (params (OverlappedComponent :type Primitive%20Component%20Object%20Reference) (OtherActor :type Actor%20Object%20Reference) (OtherComp :type Primitive%20Component%20Object%20Reference) (OtherBodyIndex :type Integer))
  (if (== OtherActor (Variables|Default|Getplayer))
    (Variables|Default|SetnearGrind false)))

(event OnComponentBeginOverlap(Trigger)
  (params (OverlappedComponent :type Primitive%20Component%20Object%20Reference) (OtherActor :type Actor%20Object%20Reference) (OtherComp :type Primitive%20Component%20Object%20Reference) (OtherBodyIndex :type Integer) (bFromSweep :type Boolean) (SweepResult :type Hit%20Result%20Structure%20%28by%20ref%29))
  (if (== OtherActor (Variables|Default|Getplayer))
    (Variables|Default|SetnearGrind true)))

(event Custom|OnGrindstoneBegin
  (params (Tool :type BP%20Test%20Tool%20Base%20Object%20Reference))
  (if (not (Variables|Default|GetinMinigame))
    (Variables|Default|SetplayersTool Tool)
    (Development|PrintString "grindStone Minigame")
    (Utilities|FlowControl|Sequence
      (:then_0
        (Variables|Default|SetcurrentTime (Utilities|Time|GetTimeSeconds))
        (Variables|Default|SetgrindTime 0.0))
      (:then_1
        (Variables|Default|SetNewProgress (/ (+ (Math|Trig|Sin(Degrees) (* (Variables|Default|GetcurrentTime) (Variables|Default|GetbarSpeed))) 1.0) 2.0)))
      (:then_2
        (bind _output_get (Variables|Default|SetNewAngle (Math|Float|Lerp 0.0 1.0 (Variables|Default|GetNewProgress))))
        (bind _returnvalue (UserInterface|CreateWidget "/Game/CustomerInteractions/UI/WB_GrindstoneUI.WB_GrindstoneUI_C" (Game|GetPlayerController 0) _output_get)) ; TODO: Needs to be removed from screen at some point
        (UserInterface|Viewport|AddtoViewport _returnvalue 0)
        (Variables|Default|SetUI _returnvalue)
        (Variables|Default|SetinMinigame true)))))

(event Custom|StartGrinding
  (bind _ui (Variables|Default|GetUI))
  (bind _ui_2 (Variables|Default|GetUI))
  (bind _clickarea (Variables|/Game/CustomerInteractions/UI/WB_GrindstoneUI.WB_GrindstoneUI_C|GetClickArea _ui))
  (bind _progress (Variables|/Game/CustomerInteractions/UI/WB_GrindstoneUI.WB_GrindstoneUI_C|GetProgress _ui_2))
  (bind _returnvalue (Class|Widget|GetRenderTransformAngle _clickarea))
  (if (== (Variables|Default|GetgrindTime) 0.0)
    (Variables|Default|SetgrindTime 0.1)
    (Variables|Default|SetcurrentTime (Utilities|Time|GetTimeSeconds))
    (else
      (Variables|Default|SetgrindTime (+ (Variables|Default|GetgrindTime) (- (Utilities|Time|GetTimeSeconds) (Variables|Default|GetcurrentTime))))
      (Variables|Default|SetcurrentTime (Utilities|Time|GetTimeSeconds))))
  (Utilities|IsValid (Variables|Default|GetplayersTool)
    (:Is%20Valid
      (Transformation|SetWorldLocation (Variables|/Game/QuenchingMinigame/BP_TestToolBase.BP_TestToolBase_C|GetDefaultSceneRoot (Variables|Default|GetplayersTool)) (Transformation|GetWorldLocation (Variables|Default|GetTop1)) false false))
    (:Is%20Not%20Valid
      _))
  (if (Math|Float|InRange(Float) (* (Variables|Default|GetNewAngle) 3.6e+02) _returnvalue (+ _returnvalue (* (Variables|/Game/CustomerInteractions/UI/WB_GrindstoneBar.WB_GrindstoneBar_C|GetPercent _clickarea) 3.6e+02)))
    (Variables|/Script/UMG.UserWidget|SetColorAndOpacity _progress "(R=0.046952,G=0.302083,B=0.000000,A=1.000000)")
    (else
      (Variables|/Script/UMG.UserWidget|SetColorAndOpacity _progress "(R=0.854167,G=0.056164,B=0.000000,A=1.000000)"))))

(event Custom|OnGrindstoneEnd
  (Widget|RemovefromParent (Variables|Default|GetUI))
  (Variables|Default|SetinMinigame false))

(event Custom|StopGrinding
  (Utilities|IsValid (Variables|Default|GetplayersTool)
    (:Is%20Valid
      (Transformation|SetWorldLocation (Variables|/Game/QuenchingMinigame/BP_TestToolBase.BP_TestToolBase_C|GetDefaultSceneRoot (Variables|Default|GetplayersTool)) (Transformation|GetWorldLocation (Variables|Default|GetTop)) false false))
    (:Is%20Not%20Valid
      _))
  (Variables|/Script/UMG.UserWidget|SetColorAndOpacity (Variables|/Game/CustomerInteractions/UI/WB_GrindstoneUI.WB_GrindstoneUI_C|GetProgress (Variables|Default|GetUI)) "(R=1.000000,G=1.000000,B=1.000000,A=1.000000)"))

(event EventTick
  (params (DeltaSeconds :type Float%20%28single-precision%29))
  (if (Variables|Default|GetinMinigame)
    (if (>= (Variables|Default|GetgrindTime) (Variables|Default|GetmaxGrindTime))
      (CallFunction|OnGrindstoneEnd)
      (else
        (Utilities|FlowControl|Sequence
          (:then_0
            (if (or (>= (+ (Variables|Default|GetNewProgress) (* DeltaSeconds (Variables|Default|GetbarSpeed))) 1.0) (<= (+ (Variables|Default|GetNewProgress) (* DeltaSeconds (Variables|Default|GetbarSpeed))) 0.0))
              (Variables|Default|SetbarSpeed (* (Variables|Default|GetbarSpeed) -1.0))
              (else
                (Variables|Default|SetNewProgress (+ (Variables|Default|GetNewProgress) (* DeltaSeconds (Variables|Default|GetbarSpeed)))))))
          (:then_1
            (bind _output_get (Variables|Default|SetNewAngle (Math|Float|Lerp 0.0 1.0 (Variables|Default|GetNewProgress))))
            (Variables|/Game/CustomerInteractions/UI/WB_GrindstoneBar.WB_GrindstoneBar_C|SetPercent (Variables|/Game/CustomerInteractions/UI/WB_GrindstoneUI.WB_GrindstoneUI_C|GetProgress (Variables|Default|GetUI)) _output_get)))))))

(event EventBeginPlay
  (bind _asbp_first_person_character (Utilities|Casting|CastToBP_FirstPersonCharacter (Game|Player|GetPlayerPawn 0)))
  (Variables|Default|Setplayer _asbp_first_person_character))

(fn ConstructionScript)